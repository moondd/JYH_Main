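; BP_WorkPoint is a work spot actor where one JYH_BP_Character_Base character works, optionally playing a looping animation.
; StartWorking stores and notifies the character, turns it toward the point or matches CharacterPoint's rotation per LookAt, optionally snaps location, and plays WorkAnimation in single-node mode.
; LeaveWork restores the Animation Blueprint and its cached instance, then ends work and clears the character.
; IsPointAnimationPlay, despite its name, returns true when no valid character occupies the point.
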(event Custom|StartWorking
  (params (Pawn :type Pawn%20Object%20Reference))
  (bind _characterpoint (Variables|Default|GetCharacterPoint))
  (bind _workanimation (Variables|Default|GetWorkAnimation))
  (bind _asjyh_bp_character_base (Utilities|Casting|CastToJYH_BP_Character_Base Pawn))
  (bind _output_get (Variables|Default|SetCurrCharacter _asjyh_bp_character_base))
  (Default|WorkStart _output_get self)
  (Utilities|FlowControl|Sequence
    (:then_0
      (switch Utilities|FlowControl|Switch|SwitchonE_FaceToOnWorkPoint (Variables|Default|GetLookAt)
        (:NewEnumerator1
          (Transformation|SetActorRotation _output_get (Math|Rotator|MakeRotator 0.0 0.0 (.Yaw (Math|Rotator|BreakRotator (Math|Rotator|FindLookatRotation (Transformation|GetActorLocation _output_get) (Transformation|GetActorLocation)))))))
        (:NewEnumerator2
          (Transformation|SetActorRotation _output_get (Transformation|GetWorldRotation _characterpoint)))))
    (:then_1
      (if (Variables|Default|GetLockLocation)
        (Transformation|SetActorLocation (Variables|Default|GetCurrCharacter) (Transformation|GetWorldLocation _characterpoint) false false)))
    (:then_2
      (Utilities|IsValid _workanimation
        (:Is%20Valid
          (Components|Animation|SetAnimationMode (Variables|/Script/Engine.Character|GetMesh _output_get) "AnimationSingleNode")
          (Components|Animation|PlayAnimation (Variables|/Script/Engine.Character|GetMesh _output_get) _workanimation true))))))

(event Custom|LeaveWork
  (Utilities|FlowControl|Sequence
    (:then_0
      (Utilities|IsValid (Variables|Default|GetWorkAnimation)
        (:Is%20Valid
          (Components|Animation|SetAnimationMode (Variables|/Script/Engine.Character|GetMesh (Variables|Default|GetCurrCharacter)) "AnimationBlueprint")
          (bind _asjyh_anim_bp_character (Utilities|Casting|CastToJYH_AnimBP_Character (Components|SkeletalMesh|GetAnimInstance (Variables|/Script/Engine.Character|GetMesh (Variables|Default|GetCurrCharacter)))))
          (Variables|/Game/MyGame/GameMode/Character/JYH_BP_Character_Base.JYH_BP_Character_Base_C|SetAnimInstance (Variables|Default|GetCurrCharacter) _asjyh_anim_bp_character))))
    (:then_1
      (Default|WorkEnd (Variables|Default|GetCurrCharacter))
      (Variables|Default|SetCurrCharacter 0))))

(event EventBeginPlay)

(event Collision|EventActorBeginOverlap
  (params (OtherActor :type Actor%20Object%20Reference)))

(event EventTick
  (params (DeltaSeconds :type Float%20%28single-precision%29)))

(fn ConstructionScript)

(fn IsPointAnimationPlay
  (Utilities|IsValid (Variables|Default|GetCurrCharacter)
    (:Is%20Valid
      (return false))
    (:Is%20Not%20Valid
      (return true))))