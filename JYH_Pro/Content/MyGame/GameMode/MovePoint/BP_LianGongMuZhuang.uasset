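; BP_LianGongMuZhuang is a martial-arts training dummy work point that characters can start and leave.
; When a player-controlled pawn starts working, it switches the player controller's UI mode and sets the current character's health to the MaxHealth from its guild and character ID data.
; On leaving, it switches a player-controlled character's UI to another mode before the parent class finishes the exit.
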(event EventBeginPlay
  (|CallParentFunction) ; This node is disabled and will not be called.\nDrag off pins to build functionality.
)

(event Collision|EventActorBeginOverlap
  (params (OtherActor :type Actor%20Object%20Reference))
  (|CallParentFunction OtherActor) ; This node is disabled and will not be called.\nDrag off pins to build functionality.
)

(event EventTick
  (params (DeltaSeconds :type Float%20%28single-precision%29))
  (|CallParentFunction DeltaSeconds) ; This node is disabled and will not be called.\nDrag off pins to build functionality.
)

(event EventStartWorking
  (params (Pawn :type Pawn%20Object%20Reference))
  (bind _currcharacter (Variables|Default|GetCurrCharacter))
  (|CallParentFunction Pawn)
  (Utilities|IsValid Pawn
    (:Is%20Valid
      (if (Pawn|IsPlayerControlled Pawn)
        (bind _asjyh_bp_player_controller (Utilities|Casting|CastToJYH_BP_PlayerController (Pawn|GetController Pawn)))
        (Default|CEChangeUI _asjyh_bp_player_controller "NewEnumerator5")
        (bind _maxhealth (CallFunction|UnexpectedCharacterData (CallFunction|GetCharacterData (Variables|/Game/MyGame/GameMode/Character/JYH_BP_Character_Base.JYH_BP_Character_Base_C|GetCharacterGuildID _currcharacter) (Variables|/Game/MyGame/GameMode/Character/JYH_BP_Character_Base.JYH_BP_Character_Base_C|GetCharacterChildID _currcharacter))))
        (Default|SetCharacterHealth _currcharacter _maxhealth)))))

(event EventLeaveWork
  (bind _currcharacter (Variables|Default|GetCurrCharacter))
  (Utilities|IsValid _currcharacter
    (:Is%20Valid
      (if (Pawn|IsPlayerControlled _currcharacter)
        (bind _asjyh_bp_player_controller (Utilities|Casting|CastToJYH_BP_PlayerController (Pawn|GetController _currcharacter))
          (:then
            (Default|CEChangeUI _asjyh_bp_player_controller "NewEnumerator4"))
          (:CastFailed
            _))))
    (:Is%20Not%20Valid
      _))
  (|CallParentFunction))

(fn ConstructionScript
  (|CallParentFunction))