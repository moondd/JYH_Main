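; Shared function library for a wuxia game, covering character generation, guild relations, items and UI popups, including guild-war choices.
; Guild and character records live in SaveGame arrays, addressed by index or "GuildID,ChildID" strings.
; Random characters get DataTable names and guild-based gear; combat stats derive from attributes and per-level GestMap growth.
; Occupations and social roles follow guild type and member index, while camp and moral matchups score character affinity.
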(fn RandomCharacterDataCreat
  (params (Camp :type E_Camp%20Enum :default "NewEnumerator0") (Moral :type E_Moral%20Enum :default "NewEnumerator0") (GuildData :type S%20Guild%20Data%20Structure))
  (bind (_guildtype _name) (Utilities|Struct|BreakS_GuildData GuildData))
  (bind (_surname _name_2) (CallFunction|RandomCharacterName))
  (Utilities|FlowControl|Sequence
    (:then_0
      ;[1 1 1] 根据类型生成装备
      (switch Utilities|FlowControl|Switch|SwitchonE_GuildType _guildtype
        (:NewEnumerator0
          (Utilities|FlowControl|Sequence :!label _label
            (:then_0
              (switch int (Math|Random|RandomIntegerinRange 0 5)
                (:0
                  (LocalVariables|SetWeapon "铁枪" :!label _label_2)
                  (LocalVariables|SetBody "长袖布袍")
                  (LocalVariables|SetLeg "布裤"))
                (:1
                  (LocalVariables|SetWeapon "铁剑" :!label _label_3)
                  (LocalVariables|SetBody "中袖布衣")
                  (LocalVariables|SetLeg "布裤"))
                (:2
                  (LocalVariables|SetWeapon "铁剑" :!label _label_4)
                  (LocalVariables|SetBody "长袖布袍")
                  (LocalVariables|SetLeg "布裤"))
                (:3
                  (LocalVariables|SetWeapon "精铁双剑" :!label _label_5)
                  (LocalVariables|SetBody "长袖布袍")
                  (LocalVariables|SetLeg "布裤"))
                (:4
                  (LocalVariables|SetWeapon "钢刀" :!label _label_6)
                  (LocalVariables|SetBody "中袖衫")
                  (LocalVariables|SetLeg "布裤"))
                (:5
                  (LocalVariables|SetBody "中袖衫" :!label _label_7)
                  (LocalVariables|SetLeg "布裤"))))
            (:then_1
              (if (Math|Random|RandomBool)
                (LocalVariables|SetBody "None")))))
        (:NewEnumerator5
          (goto _label))
        (:NewEnumerator3
          (goto _label))
        (:NewEnumerator1
          (goto _label))
        (:NewEnumerator4
          (goto _label))
        (:NewEnumerator2
          (Utilities|FlowControl|Sequence
            (:then_0
              (switch name _name
                (:圣龙坛
                  (goto _label_2))
                (:青城派
                  (goto _label_3))
                (:龙华寺
                  (goto _label_7))
                (:全真教
                  (goto _label_4))
                (:黄山
                  (goto _label_5))
                (:日月教
                  (goto _label_5))
                (:朝廷
                  (goto _label_6))
                (:华山派
                  (goto _label_3))
                (:武当派
                  (goto _label_4))
                (:少林寺
                  (goto _label_7))
                (:天命门
                  (goto _label_2))
                (:丐帮
                  (goto _label_2))
                (:逍遥派
                  (goto _label_4))))
            (:then_1
              (if (Math|Random|RandomBool)
                (LocalVariables|SetHat "毡帽")))))))
    (:then_1
      (bind _maxhealth (CallFunction|UnexpectedCharacterData (Utilities|Struct|MakeS_CharacterData _surname _name_2 Camp Moral 0 0 0 0 0 1.2e+02 "NewEnumerator0" false (Utilities|Map|MakeMap "银两" (Math|Random|RandomIntegerinRange 1 24)) (Utilities|Map|MakeMap "Weapon" (LocalVariables|GetWeapon) "Hat" (LocalVariables|GetHat) "Body" (LocalVariables|GetBody) "Leg" (LocalVariables|GetLeg)))))
      (bind _structout (Utilities|Struct|SetmembersinS_CharacterData (Utilities|Struct|MakeS_CharacterData _surname _name_2 Camp Moral 0 0 0 0 0 1.2e+02 "NewEnumerator0" false (Utilities|Map|MakeMap "银两" (Math|Random|RandomIntegerinRange 1 24)) (Utilities|Map|MakeMap "Weapon" (LocalVariables|GetWeapon) "Hat" (LocalVariables|GetHat) "Body" (LocalVariables|GetBody) "Leg" (LocalVariables|GetLeg))) _maxhealth))
      (return _structout))))

(fn GetMyGameInstance
  (bind _asbp_game_instance (Utilities|Casting|CastToBP_GameInstance (Game|GetGameInstance)))
  (return _asbp_game_instance))

(fn GetMySaveGame
  (return (Variables|/Game/MyGame/GameMode/Buleprint/BP_GameInstance.BP_GameInstance_C|GetSaveGame (CallFunction|GetMyGameInstance))))

(fn GetGuildXY
  (params (InGuildID :type Integer) (InWeight :type Integer))
  (bind _returnvalue (/ InGuildID InWeight))
  (return (- InGuildID (* _returnvalue InWeight)) _returnvalue))

(fn GetGuildDatawithID
  (params (ID :type Integer))
  (bind _newparam (CallFunction|GetMySaveGame))
  (bind _guilddataarray (Variables|/Game/MyGame/GameMode/Buleprint/BP_SaveGame.BP_SaveGame_C|GetGuildDataArray _newparam))
  (if (Utilities|Array|IsValidIndex _guilddataarray ID)
    (return (Utilities|Array|Get(acopy) _guilddataarray ID))
    (else
      (Development|PrintString 0 (Utilities|String|JoinStringArray (Utilities|Array|MakeArray "GetGuildData失败:" "Guild " (Utilities|String|ToString(Integer) ID)) " ") true true "(R=1.000000,G=0.000000,B=0.000000,A=1.000000)")
      (return (Utilities|Struct|MakeS_GuildData)))))

(fn GuildXYtoID
  (params (X :type Integer) (Y :type Integer) (Weight :type Integer))
  (return (+ (* Y Weight) X)))

(fn RandomCharacterName
  (Utilities|FlowControl|Sequence
    (:then_0
      (bind _outrownames (DataTable|GetDataTableRowNames "/Game/MyGame/GameMode/GameData/DT_Surname.DT_Surname"))
      (bind _returnvalue (Utilities|GetDataTableRow "/Game/MyGame/GameMode/GameData/DT_Surname.DT_Surname" (Utilities|Array|Get(acopy) _outrownames (Math|Random|RandomIntegerinRange 0 (Utilities|Array|LastIndex _outrownames))))
        (:RowNotFound
          _)))
    (:then_1
      (bind _outrownames_2 (DataTable|GetDataTableRowNames "/Game/MyGame/GameMode/GameData/DT_Name_Male.DT_Name_Male"))
      (bind _returnvalue_2 (Utilities|GetDataTableRow "/Game/MyGame/GameMode/GameData/DT_Name_Male.DT_Name_Male" (Utilities|Array|Get(acopy) _outrownames_2 (Math|Random|RandomIntegerinRange 0 (Utilities|Array|LastIndex _outrownames_2))))
        (:RowNotFound
          _)))
    (:then_2
      (return (Utilities|Struct|BreakS_Text _returnvalue) (Utilities|Struct|BreakS_Text _returnvalue_2))))
  (return "无" "名"))

(fn GetCharacterOcc
  (params (GuildType :type E_GuildType%20Enum :default "NewEnumerator0") (Faith :type E_Faith%20Enum :default "NewEnumerator0") (CharacterChildID :type Integer))
  (switch Utilities|FlowControl|Switch|SwitchonE_GuildType GuildType
    (:NewEnumerator0
      _)
    (:NewEnumerator5
      _)
    (:NewEnumerator3
      _)
    (:NewEnumerator1
      _)
    (:NewEnumerator4
      _)
    (:NewEnumerator2
      (switch Utilities|FlowControl|Switch|SwitchonE_Faith Faith
        (:NewEnumerator0
          (switch int CharacterChildID
            (:Default
              (return "NewEnumerator10"))
            (:0
              (return "NewEnumerator5"))
            (:1
              (return "NewEnumerator6"))
            (:2
              (return "NewEnumerator7"))
            (:3
              (return "NewEnumerator8"))
            (:4
              _)
            (:5
              _)
            (:6
              _))
          (return "NewEnumerator9"))
        (:NewEnumerator1
          (switch int CharacterChildID
            (:Default
              (return "NewEnumerator22"))
            (:0
              (return "NewEnumerator17"))
            (:1
              (return "NewEnumerator19"))
            (:2
              (return "NewEnumerator20"))
            (:3
              (return "NewEnumerator18"))
            (:4
              _)
            (:5
              _)
            (:6
              _))
          (return "NewEnumerator21"))
        (:NewEnumerator2
          (switch int CharacterChildID
            (:Default
              (return "NewEnumerator16"))
            (:0
              (return "NewEnumerator11"))
            (:1
              (return "NewEnumerator12"))
            (:2
              (return "NewEnumerator13"))
            (:3
              (return "NewEnumerator15"))
            (:4
              _)
            (:5
              _)
            (:6
              _))
          (return "NewEnumerator14")))))
  (return "NewEnumerator0"))

(fn GetParentGuildID
  (params (GuildID :type Integer))
  (return (.ParentGuildID (Utilities|Struct|BreakS_GuildData (CallFunction|GetGuildDatawithID GuildID)))))

(fn GetCharacterData
  (params (GuildID :type Integer) (CharacterID :type Integer))
  (bind _newparam (CallFunction|GetMySaveGame))
  (bind _guilddataarray (Variables|/Game/MyGame/GameMode/Buleprint/BP_SaveGame.BP_SaveGame_C|GetGuildDataArray _newparam))
  (bind _output (Utilities|Array|Get(acopy) _guilddataarray GuildID))
  (bind _characterdataarray (Utilities|Struct|BreakS_GuildData _output))
  (if (Utilities|Array|IsValidIndex _guilddataarray GuildID)
    (if (Utilities|Array|IsValidIndex _characterdataarray CharacterID)
      (return (Utilities|Array|Get(acopy) _characterdataarray CharacterID))
      (else
        _)))
  (Development|PrintString 0 (Utilities|String|JoinStringArray (Utilities|Array|MakeArray "角色数据丢失" (Utilities|String|ToString(Integer) GuildID) (Utilities|String|ToString(Integer) CharacterID)) " ") true true "(R=1.000000,G=0.000000,B=0.000000,A=1.000000)")
  (return (Utilities|Struct|MakeS_CharacterData 0 0 0.0)))

(fn UnexpectedCharacterData
  (params (CharacterData :type S%20Character%20Data%20Structure))
  (bind (_surname _name _camp _moral _exp _constitution _strength _dexterous _intelligence _currhealth _occ _ismission_ _itemmap _equipmap _gestmap) (Utilities|Struct|BreakS_CharacterData CharacterData))
  (Utilities|FlowControl|Sequence
    (:then_0
      (bind _keys (Utilities|Map|Keys _gestmap))
      (for _array_element _keys
        (bind _returnvalue (Utilities|GetDataTableRow "/Game/MyGame/GameMode/GameData/DT_GestData.DT_GestData" _array_element)
          (:then
            (LocalVariables|SetLoc_Con (+ (LocalVariables|GetLoc_Con) (* (Math|Conversions|ToInteger(Byte) (Utilities|Array|Get(acopy) (Utilities|String|ParseIntoArray (.LevelUpValue (Utilities|Struct|BreakS_GestData _returnvalue)) ","))) (.Value (Utilities|Map|Find _gestmap _array_element)))))
            (LocalVariables|SetLoc_Str (+ (LocalVariables|GetLoc_Str) (* (Math|Conversions|ToInteger(Byte) (Utilities|Array|Get(acopy) (Utilities|String|ParseIntoArray (.LevelUpValue (Utilities|Struct|BreakS_GestData _returnvalue)) ",") 1)) (.Value (Utilities|Map|Find _gestmap _array_element)))))
            (LocalVariables|SetLoc_Dex (+ (LocalVariables|GetLoc_Dex) (* (Math|Conversions|ToInteger(Byte) (Utilities|Array|Get(acopy) (Utilities|String|ParseIntoArray (.LevelUpValue (Utilities|Struct|BreakS_GestData _returnvalue)) ",") 2)) (.Value (Utilities|Map|Find _gestmap _array_element)))))
            (LocalVariables|SetLoc_Int (+ (LocalVariables|GetLoc_Int) (* (Math|Conversions|ToInteger(Byte) (Utilities|Array|Get(acopy) (Utilities|String|ParseIntoArray (.LevelUpValue (Utilities|Struct|BreakS_GestData _returnvalue)) ",") 3)) (.Value (Utilities|Map|Find _gestmap _array_element)))))))))
    (:then_1
      (LocalVariables|SetLoc_QiXue (+ (+ 1.2e+02 (* _constitution 0.6)) (* (LocalVariables|GetLoc_Con) (CallFunction|CalculateGrowValue _constitution 1.2))))
      (LocalVariables|SetLoc_GongJi (+ (+ 3e+01 (* _strength 0.15)) (* (LocalVariables|GetLoc_Str) (CallFunction|CalculateGrowValue _strength 0.3))))
      (LocalVariables|SetLoc_HuaJie (/ 1.0 (+ (+ 1.0 (* _dexterous 0.005)) (* (LocalVariables|GetLoc_Dex) (CallFunction|CalculateGrowValue _dexterous 0.01)))))
      (LocalVariables|SetLoc_JiaCheng (+ (+ 1.0 (* _intelligence 0.005)) (* (LocalVariables|GetLoc_Int) (CallFunction|CalculateGrowValue _intelligence 0.01)))))
    (:then_2
      (return (LocalVariables|GetLoc_QiXue) (* (LocalVariables|GetLoc_GongJi) (LocalVariables|GetLoc_JiaCheng)) (LocalVariables|GetLoc_HuaJie) (+ (/ (LocalVariables|GetLoc_QiXue) 1.2e+02) (/ (LocalVariables|GetLoc_GongJi) 3e+01) (/ 1.0 (LocalVariables|GetLoc_HuaJie)) (/ (LocalVariables|GetLoc_JiaCheng) 1.0))))))

(fn GetGameModeWorldMap
  (bind _asbp_game_mode_world_map (Utilities|Casting|CastToBP_GameMode_WorldMap (Game|GetGameMode))
    (:then
      (return _asbp_game_mode_world_map))
    (:CastFailed
      (return 0))))

(fn AddItemtoCharacterData
  (params (CharacterData :type S%20Character%20Data%20Structure%20%28by%20ref%29) (ItemName :type Name))
  (bind _itemmap (Utilities|Struct|BreakS_CharacterData CharacterData))
  (if (Utilities|Name|NotEqual(Name) ItemName "None")
    (if (Utilities|Map|Contains _itemmap ItemName)
      (Utilities|Map|Add _itemmap ItemName (+ (.Value (Utilities|Map|Find _itemmap ItemName)) 1))
      (else
        (Utilities|Map|Add _itemmap ItemName 1)))))

(fn RemoveIteminCharacterData
  (params (CharacterData :type S%20Character%20Data%20Structure%20%28by%20ref%29) (ItemName :type Name))
  (bind _itemmap (Utilities|Struct|BreakS_CharacterData CharacterData))
  (bind _value (Utilities|Map|Find _itemmap ItemName))
  (if (Utilities|Map|Contains _itemmap ItemName)
    (Utilities|Map|Add _itemmap ItemName (- _value 1))
    (if (<= _value 0)
      (Utilities|Map|Remove _itemmap ItemName))))

(fn FindIteminCharacterItems
  (params (Item :type S%20Item%20Structure) (ItemArray :type Array%20of%20S%20Item%20Structures))
  (for (_array_element _array_index) ItemArray
    (if (Utilities|Enum|Equal(Enum) (.Name (Utilities|Struct|BreakS_Item _array_element)) (.Name (Utilities|Struct|BreakS_Item Item)))
      (return _array_index true)))
  (return 0 false))

(fn ShowPopSelectWindow
  (params (Info :type Text) (ButtonTextArray :type Map%20of%20Strings%20to%20Booleans))
  (bind _returnvalue (UserInterface|CreateWidget "/Game/MyGame/UI/W_PopSelect.W_PopSelect_C"))
  (Default|SetPopText _returnvalue Info ButtonTextArray)
  (UserInterface|Viewport|AddtoPlayerScreen _returnvalue 10)
  (return _returnvalue))

(fn ShowGameInfo
  (params (GameInfo :type Text))
  (bind _asjyh_bp_player_controller (Utilities|Casting|CastToJYH_BP_PlayerController (Game|GetPlayerController 0)))
  (Default|ShowGameInfo (Variables|/Game/MyGame/GameMode/Character/JYH_BP_PlayerController.JYH_BP_PlayerController_C|GetInGame _asjyh_bp_player_controller) GameInfo))

(fn CharacterIDtoString
  (params (GuildID :type Integer) (ChildID :type Integer))
  (return (Utilities|String|JoinStringArray (Utilities|Array|MakeArray (Utilities|String|ToString(Integer) GuildID) (Utilities|String|ToString(Integer) ChildID)) ",")))

(fn CalculateGrowValue
  (params (Int :type Integer) (GrowValue :type Float%20%28single-precision%29))
  (return (+ GrowValue (* (/ (Math|Conversions|ToFloat(Integer) Int) 1e+02) GrowValue))))

(fn TwoCharacterFriendVelue
  (params (InCharacterData_0 :type S%20Character%20Data%20Structure) (InCharacterData_1 :type S%20Character%20Data%20Structure))
  (bind (_camp _moral) (Utilities|Struct|BreakS_CharacterData InCharacterData_0))
  (bind (_camp_2 _moral_2) (Utilities|Struct|BreakS_CharacterData InCharacterData_1))
  (Utilities|FlowControl|Sequence
    (:then_0
      (switch Utilities|FlowControl|Switch|SwitchonE_Camp _camp
        (:NewEnumerator0
          (switch Utilities|FlowControl|Switch|SwitchonE_Camp _camp_2
            (:NewEnumerator0
              (LocalVariables|SetLocalVar_CampPoint 100 :!label _label))
            (:NewEnumerator1
              (LocalVariables|SetLocalVar_CampPoint -100 :!label _label_2))
            (:NewEnumerator2
              (LocalVariables|SetLocalVar_CampPoint 0 :!label _label_3))))
        (:NewEnumerator1
          (switch Utilities|FlowControl|Switch|SwitchonE_Camp _camp_2
            (:NewEnumerator0
              (goto _label_3))
            (:NewEnumerator1
              (goto _label))
            (:NewEnumerator2
              (goto _label_2))))
        (:NewEnumerator2
          (switch Utilities|FlowControl|Switch|SwitchonE_Camp _camp_2
            (:NewEnumerator0
              (goto _label_2))
            (:NewEnumerator1
              (goto _label_3))
            (:NewEnumerator2
              (goto _label))))))
    (:then_1
      (switch Utilities|FlowControl|Switch|SwitchonE_Moral _moral
        (:NewEnumerator0
          (switch Utilities|FlowControl|Switch|SwitchonE_Moral _moral_2
            (:NewEnumerator0
              (LocalVariables|SetLocalVar_MoralPoint 100 :!label _label_4))
            (:NewEnumerator8
              (LocalVariables|SetLocalVar_MoralPoint 0 :!label _label_5))
            (:NewEnumerator9
              (LocalVariables|SetLocalVar_MoralPoint -100 :!label _label_6))))
        (:NewEnumerator8
          (switch Utilities|FlowControl|Switch|SwitchonE_Moral _moral_2
            (:NewEnumerator0
              (goto _label_6))
            (:NewEnumerator8
              (goto _label_4))
            (:NewEnumerator9
              (goto _label_5))))
        (:NewEnumerator9
          (switch Utilities|FlowControl|Switch|SwitchonE_Moral _moral_2
            (:NewEnumerator0
              (goto _label_5))
            (:NewEnumerator8
              (goto _label_6))
            (:NewEnumerator9
              (goto _label_4))))))
    (:then_2
      (return (+ (LocalVariables|GetLocalVar_CampPoint) (LocalVariables|GetLocalVar_MoralPoint))))))

(fn CharacterJoinNewGuild
  (params (CharacterGuildID :type Integer) (CharacterChildID :type Integer) (NewGuildID :type Integer) (Character :type JYH%20BP%20Character%20Base%20Object%20Reference))
  (bind _newparam (CallFunction|GetMySaveGame))
  (bind _guilddataarray (Variables|/Game/MyGame/GameMode/Buleprint/BP_SaveGame.BP_SaveGame_C|GetGuildDataArray _newparam))
  (LocalVariables|SetLoc_OldGuildID CharacterGuildID)
  (LocalVariables|SetLoc_OldChildID CharacterChildID)
  (bind _output_get (LocalVariables|SetLoc_NewGuildID NewGuildID))
  (bind _returnvalue (Utilities|Array|Add (.CharacterDataArray (Utilities|Struct|BreakS_GuildData (Utilities|Array|Get(acopy) _guilddataarray _output_get))) (CallFunction|GetCharacterData (LocalVariables|GetLoc_OldGuildID) (LocalVariables|GetLoc_OldChildID))))
  (LocalVariables|SetLoc_NewChildID _returnvalue)
  (Utilities|Array|RemoveItem (.CharacterDataArray (Utilities|Struct|BreakS_GuildData (Utilities|Array|Get(acopy) _guilddataarray (LocalVariables|GetLoc_OldGuildID)))) (Utilities|Array|Get(acopy) (.CharacterDataArray (Utilities|Struct|BreakS_GuildData (Utilities|Array|Get(acopy) _guilddataarray (LocalVariables|GetLoc_OldGuildID)))) (LocalVariables|GetLoc_OldChildID)))
  (Utilities|IsValid Character
    (:Is%20Valid
      (Variables|/Game/MyGame/GameMode/Character/JYH_BP_Character_Base.JYH_BP_Character_Base_C|SetCharacterGuildID Character (LocalVariables|GetLoc_NewGuildID))
      (Variables|/Game/MyGame/GameMode/Character/JYH_BP_Character_Base.JYH_BP_Character_Base_C|SetCharacterChildID Character (LocalVariables|GetLoc_NewChildID))
      (Utilities|Casting|CastToJYH_BP_Character_Player Character)
      (Variables|/Game/MyGame/GameMode/Buleprint/BP_SaveGame.BP_SaveGame_C|SetPlayerGuildID _newparam (LocalVariables|GetLoc_NewGuildID))
      (Variables|/Game/MyGame/GameMode/Buleprint/BP_SaveGame.BP_SaveGame_C|SetPlayerChildID _newparam (LocalVariables|GetLoc_NewChildID)))))

(fn RetrunCharacterSocial
  (params (CharacterString0 :type String) (CharacterString1 :type String))
  (bind (_characterguildid _characterchildid) (CallFunction|CharacterStringtoID CharacterString1))
  (bind (_characterguildid_2 _characterchildid_2) (CallFunction|CharacterStringtoID CharacterString0))
  (if (Utilities|Enum|Equal(Enum) (.GuildType (Utilities|Struct|BreakS_GuildData (CallFunction|GetGuildDatawithID _characterguildid_2))) "NewEnumerator2")
    (if (== _characterguildid_2 _characterguildid)
      (return (select (<= _characterchildid 2) (Utilities|Select :Index _characterchildid :Option%200 "NewEnumerator24" :Option%201 "NewEnumerator25" :Option%202 "NewEnumerator26") (select (> _characterchildid_2 _characterchildid) "NewEnumerator28" "NewEnumerator27")))
      (else
        _)))
  (return (.Occ (Utilities|Struct|BreakS_CharacterData (CallFunction|GetCharacterData _characterguildid _characterchildid)))))

(fn CharacterStringtoID
  (params (CharacterString :type String))
  (bind _returnvalue (Utilities|String|ParseIntoArray CharacterString ","))
  (if (and (Utilities|Array|IsValidIndex _returnvalue) (Utilities|Array|IsValidIndex _returnvalue 1))
    (return (Math|Conversions|ToInteger(Byte) (Utilities|Array|Get(acopy) _returnvalue)) (Math|Conversions|ToInteger(Byte) (Utilities|Array|Get(acopy) _returnvalue 1)))
    (else
      (Development|PrintString 0 "获取角色ID失败CharacterStringToID" true true "(R=1.000000,G=0.000000,B=0.000000,A=1.000000)")
      (return 0 0))))

(fn AddGuildPlayerFriendValue
  (params (GuildID :type Integer) (Value :type Integer) (IsSet? :type Boolean))
  (bind _newparam (CallFunction|GetMySaveGame))
  (bind _guilddataarray (Variables|/Game/MyGame/GameMode/Buleprint/BP_SaveGame.BP_SaveGame_C|GetGuildDataArray _newparam))
  (bind _output (Utilities|Array|Get(acopy) _guilddataarray GuildID))
  (bind (_name _playerfriendvalue) (Utilities|Struct|BreakS_GuildData _output))
  (Utilities|Struct|SetmembersinS_GuildData _output (Math|Integer|SelectInt (Math|Integer|Clamp(Integer) Value -100 100) (Math|Integer|Clamp(Integer) (+ _playerfriendvalue Value) -100 100) IsSet?))
  (Development|PrintString 0 (Utilities|String|JoinStringArray (Utilities|Array|MakeArray "与" (Utilities|String|ToString(Name) _name) "的友好度为" (Utilities|String|ToString(Integer) _playerfriendvalue)) " "))
  (return _playerfriendvalue))

(fn GetItemData
  (params (ItemName :type Name))
  (bind _returnvalue (Utilities|GetDataTableRow "/Game/MyGame/GameMode/GameData/DT_ItemData.DT_ItemData" ItemName)
    (:then
      (return _returnvalue))))

(fn GetCurrGuildID
  (bind _gamemode (CallFunction|GetGameModeWorldMap))
  (bind _currguildpoint (Variables|/Game/MyGame/GameMode/Buleprint/BP_GameMode_WorldMap.BP_GameMode_WorldMap_C|GetCurrGuildPoint _gamemode))
  (Utilities|IsValid _currguildpoint
    (:Is%20Valid
      (return (Variables|/Game/MyGame/GameMode/Buleprint/BP_GuildPoint.BP_GuildPoint_C|GetGuildID _currguildpoint)))
    (:Is%20Not%20Valid
      (return -1))))

(fn SetGuildFriendValue
  (params (InGuildID :type Integer) (InOtherGuildID :type Integer) (Value :type Integer) (IsAdd? :type Boolean))
  (bind _newparam (CallFunction|GetMySaveGame))
  (bind _guilddataarray (Variables|/Game/MyGame/GameMode/Buleprint/BP_SaveGame.BP_SaveGame_C|GetGuildDataArray _newparam))
  (LocalVariables|SetLocalVar_GuildID InGuildID)
  (LocalVariables|SetLocalVar_TargetGuildID InOtherGuildID)
  (LocalVariables|SetLocalVar_AddValue Value)
  (if IsAdd?
    (if (Utilities|Array|IsValidIndex (.GuildFriendValueArray (Utilities|Struct|BreakS_GuildData (Utilities|Array|Get(acopy) _guilddataarray (LocalVariables|GetLocalVar_GuildID)))) (LocalVariables|GetLocalVar_TargetGuildID))
      (Utilities|Array|SetArrayElem (.GuildFriendValueArray (Utilities|Struct|BreakS_GuildData (Utilities|Array|Get(acopy) _guilddataarray (LocalVariables|GetLocalVar_GuildID)))) (LocalVariables|GetLocalVar_TargetGuildID) (+ (Utilities|Array|Get(acopy) (.GuildFriendValueArray (Utilities|Struct|BreakS_GuildData (Utilities|Array|Get(acopy) _guilddataarray (LocalVariables|GetLocalVar_GuildID)))) (LocalVariables|GetLocalVar_TargetGuildID)) (LocalVariables|GetLocalVar_AddValue)) true)
      (else
        (Utilities|Array|SetArrayElem (.GuildFriendValueArray (Utilities|Struct|BreakS_GuildData (Utilities|Array|Get(acopy) _guilddataarray (LocalVariables|GetLocalVar_GuildID)))) (LocalVariables|GetLocalVar_TargetGuildID) (LocalVariables|GetLocalVar_AddValue) true)))
    (if (Utilities|Array|IsValidIndex (.GuildFriendValueArray (Utilities|Struct|BreakS_GuildData (Utilities|Array|Get(acopy) _guilddataarray (LocalVariables|GetLocalVar_TargetGuildID)))) (LocalVariables|GetLocalVar_GuildID))
      (Utilities|Array|SetArrayElem (.GuildFriendValueArray (Utilities|Struct|BreakS_GuildData (Utilities|Array|Get(acopy) _guilddataarray (LocalVariables|GetLocalVar_TargetGuildID)))) (LocalVariables|GetLocalVar_GuildID) (+ (Utilities|Array|Get(acopy) (.GuildFriendValueArray (Utilities|Struct|BreakS_GuildData (Utilities|Array|Get(acopy) _guilddataarray (LocalVariables|GetLocalVar_TargetGuildID)))) (LocalVariables|GetLocalVar_GuildID)) (LocalVariables|GetLocalVar_AddValue)) true)
      (else
        (Utilities|Array|SetArrayElem (.GuildFriendValueArray (Utilities|Struct|BreakS_GuildData (Utilities|Array|Get(acopy) _guilddataarray (LocalVariables|GetLocalVar_TargetGuildID)))) (LocalVariables|GetLocalVar_GuildID) (LocalVariables|GetLocalVar_AddValue) true)))
    (else
      (Utilities|Array|SetArrayElem (.GuildFriendValueArray (Utilities|Struct|BreakS_GuildData (Utilities|Array|Get(acopy) _guilddataarray (LocalVariables|GetLocalVar_GuildID)))) (LocalVariables|GetLocalVar_TargetGuildID) Value true)
      (Utilities|Array|SetArrayElem (.GuildFriendValueArray (Utilities|Struct|BreakS_GuildData (Utilities|Array|Get(acopy) _guilddataarray (LocalVariables|GetLocalVar_TargetGuildID)))) (LocalVariables|GetLocalVar_GuildID) Value true))))

(fn CreatGuildWarPop
  (params (GuildWarGroup :type S%20Guild%20War%20Group%20Structure))
  (bind (_guildwartype _group_attack _group_def) (Utilities|Struct|BreakS_GuildWarGroup GuildWarGroup))
  (LocalVariables|SetLoc_GuildWarType _guildwartype)
  (LocalVariables|SetLoc_Group_Atk _group_attack)
  (LocalVariables|SetLoc_Group_Def _group_def)
  (Utilities|FlowControl|Sequence
    (:then_0
      (bind _asjyh_bp_character_player (Utilities|Casting|CastToJYH_BP_Character_Player (Game|GetPlayerCharacter 0)))
      (bind _output_get (LocalVariables|SetLoc_PlayerGuildID (Variables|/Game/MyGame/GameMode/Character/JYH_BP_Character_Base.JYH_BP_Character_Base_C|GetCharacterGuildID _asjyh_bp_character_player)))
      (if (Utilities|Array|ContainsItem (LocalVariables|GetLoc_Group_Atk) _output_get)
        (LocalVariables|SetLoc_PlayerInGroup 1)
        (elif (Utilities|Array|ContainsItem (LocalVariables|GetLoc_Group_Def) _output_get)
          (LocalVariables|SetLoc_PlayerInGroup 2))))
    (:then_1
      (LocalVariables|SetLoc_Info (Utilities|Text|ToText(String) (Utilities|Select :Index (LocalVariables|GetLoc_GuildWarType) :NewEnumerator0 (Utilities|String|JoinStringArray (Utilities|Array|MakeArray (Utilities|String|ToString(Name) (.Name (Utilities|Struct|BreakS_GuildData (CallFunction|GetGuildDatawithID (Utilities|Array|Get(acopy) (LocalVariables|GetLoc_Group_Atk)))))) "与" (Utilities|String|ToString(Name) (.Name (Utilities|Struct|BreakS_GuildData (CallFunction|GetGuildDatawithID (Utilities|Array|Get(acopy) (LocalVariables|GetLoc_Group_Def)))))) "产生冲突。") " ") :NewEnumerator1 (Utilities|String|JoinStringArray (Utilities|Array|MakeArray (Utilities|String|ToString(Name) (.Name (Utilities|Struct|BreakS_GuildData (CallFunction|GetGuildDatawithID (Utilities|Array|Get(acopy) (LocalVariables|GetLoc_Group_Def)))))) "遭到" (Utilities|String|ToString(Name) (.Name (Utilities|Struct|BreakS_GuildData (CallFunction|GetGuildDatawithID (Utilities|Array|Get(acopy) (LocalVariables|GetLoc_Group_Atk)))))) "灭门。") " ")))))
    (:then_2
      (bind _popselect (CallFunction|ShowPopSelectWindow (LocalVariables|GetLoc_Info) (Utilities|Map|MakeMap (Utilities|String|JoinStringArray (Utilities|Array|MakeArray "袭击" (Utilities|String|ToString(Name) (.Name (Utilities|Struct|BreakS_GuildData (CallFunction|GetGuildDatawithID (Utilities|Array|Get(acopy) (LocalVariables|GetLoc_Group_Atk)))))) "关系" (Utilities|String|ToString(Integer) (.PlayerFriendValue (Utilities|Struct|BreakS_GuildData (CallFunction|GetGuildDatawithID (Utilities|Array|Get(acopy) (LocalVariables|GetLoc_Group_Atk))))))) " ") (!= (Utilities|Array|Get(acopy) (LocalVariables|GetLoc_Group_Atk)) (LocalVariables|GetLoc_PlayerGuildID)) (Utilities|String|JoinStringArray (Utilities|Array|MakeArray "袭击" (Utilities|String|ToString(Name) (.Name (Utilities|Struct|BreakS_GuildData (CallFunction|GetGuildDatawithID (Utilities|Array|Get(acopy) (LocalVariables|GetLoc_Group_Def)))))) "关系" (Utilities|String|ToString(Integer) (.PlayerFriendValue (Utilities|Struct|BreakS_GuildData (CallFunction|GetGuildDatawithID (Utilities|Array|Get(acopy) (LocalVariables|GetLoc_Group_Def))))))) " ") (!= (Utilities|Array|Get(acopy) (LocalVariables|GetLoc_Group_Def)) (LocalVariables|GetLoc_PlayerGuildID)) "袖手旁观" (and (!= (Utilities|Array|Get(acopy) (LocalVariables|GetLoc_Group_Atk)) (LocalVariables|GetLoc_PlayerGuildID)) (!= (Utilities|Array|Get(acopy) (LocalVariables|GetLoc_Group_Def)) (LocalVariables|GetLoc_PlayerGuildID))))))
      (return _popselect GuildWarGroup))))