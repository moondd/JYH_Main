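; BP_GuildController is an editor-time helper that aligns NavMeshBoundsVolumes to BP_GuildPoint actors in the level.
; Its construction script uses the Build bool as a one-shot button, resetting it and gathering both actor sets.
; It pairs them by underscore-split display names, matching the point's third token to the volume's second, then moves each matched volume to its point's location.
; The event graph holds no runtime logic.
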(event EventBeginPlay)

(event Collision|EventActorBeginOverlap
  (params (OtherActor :type Actor%20Object%20Reference)))

(event EventTick
  (params (DeltaSeconds :type Float%20%28single-precision%29)))

(fn ConstructionScript
  (if (Variables|Default|GetBuild)
    (Variables|Default|SetBuild false)
    (bind _outactors (Actor|GetAllActorsOfClass "/Script/Engine.NavMeshBoundsVolume"))
    (Variables|Default|SetNavMeshs _outactors)
    (bind _outactors_2 (Actor|GetAllActorsOfClass "/Game/MyGame/GameMode/Buleprint/BP_GuildPoint.BP_GuildPoint_C"))
    (Variables|Default|SetGuildPoints _outactors_2)
    (for _array_element (Variables|Default|GetGuildPoints)
      (for _array_element_2 (Variables|Default|GetNavMeshs)
        (if (Utilities|Enum|Equal(Enum) (Utilities|Array|Get(acopy) (Utilities|String|ParseIntoArray (Utilities|GetDisplayName _array_element) "_") 2) (Utilities|Array|Get(acopy) (Utilities|String|ParseIntoArray (Utilities|GetDisplayName _array_element_2) "_") 1))
          (Transformation|SetActorLocation _array_element_2 (Transformation|GetActorLocation _array_element) false false))))))