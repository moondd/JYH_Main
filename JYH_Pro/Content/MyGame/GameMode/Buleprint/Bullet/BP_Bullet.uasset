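; BP_Bullet is a projectile actor that damages characters it overlaps and destroys itself two seconds after spawning.
; Its Capsule overlap ignores the FromCharacter that fired it and casts any other actor to JYH_BP_Character_Base.
; A successful cast receives fixed point damage along the bullet's forward vector with an empty hit result.
; The bullet is not destroyed on hit, so it persists until the timer ends.
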(event OnComponentBeginOverlap(Capsule)
  (params (OverlappedComponent :type Primitive%20Component%20Object%20Reference) (OtherActor :type Actor%20Object%20Reference) (OtherComp :type Primitive%20Component%20Object%20Reference) (OtherBodyIndex :type Integer) (bFromSweep :type Boolean) (SweepResult :type Hit%20Result%20Structure%20%28by%20ref%29))
  (if (!= OtherActor (Variables|Default|GetFromCharacter))
    (bind _asjyh_bp_character_base (Utilities|Casting|CastToJYH_BP_Character_Base OtherActor))
    (Game|Damage|ApplyPointDamage _asjyh_bp_character_base 1e+01 (Transformation|GetActorForwardVector) (Collision|MakeHitResult false false 0.0 0.0 "0, 0, 0" "0, 0, 0" "0,0,1" "0,0,1" 0 0) 0 self)))

(event EventBeginPlay
  (Utilities|FlowControl|Delay 2.0)
  (Actor|DestroyActor))

(event Collision|EventActorBeginOverlap
  (params (OtherActor :type Actor%20Object%20Reference)))

(event EventTick
  (params (DeltaSeconds :type Float%20%28single-precision%29)))

(fn ConstructionScript)