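; BP_SaveGame, by its name a save game Blueprint, provides accessors for per-guild data stored in GuildDataArray, indexed by guild ID.
; GetGuildFriendValue reads one guild's friendship value toward another from its GuildFriendValueArray.
; SetGuildIDToInGuildArray adds or removes a guild ID in a target guild's OtherGuildInThis collection, checking membership only before removal.
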(fn GetGuildFriendValue
  (params (InGuildID :type Integer) (TargetGuildID :type Integer))
  (return (Utilities|Array|Get(acopy) (.GuildFriendValueArray (Utilities|Struct|BreakS_GuildData (Utilities|Array|Get(acopy) (Variables|Default|GetGuildDataArray) InGuildID))) TargetGuildID)))

(fn SetGuildIDtoinGuildArray
  (params (InGuildID :type Integer) (InTargetGuildID :type Integer) (Remove :type Boolean))
  (bind _guilddataarray (Variables|Default|GetGuildDataArray))
  (bind _output (Utilities|Array|Get(acopy) _guilddataarray InTargetGuildID))
  (bind _otherguildinthis (Utilities|Struct|BreakS_GuildData _output))
  (if Remove
    (if (Utilities|Array|ContainsItem _otherguildinthis InGuildID)
      (Utilities|Array|RemoveItem _otherguildinthis InGuildID))
    (else
      (Utilities|Array|Add _otherguildinthis InGuildID))))