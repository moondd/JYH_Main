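; World-map guild point actor that represents one guild location and spawns that guild's AI characters.
; Construction picks the billboard icon from GuildID and gathers tagged move points; BuildGuildShpere tints, scales and ground-snaps the sphere.
; Enter/leave events notify BP_GameMode_WorldMap, with a retreat-confirmation popup.
; AddCharacterInThisGuild spawns eligible saved characters at navigable entrance, fixed or move points with fallbacks, optionally teaming them, and registers each with the game mode.
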(event Custom|CE_SelectWhenPlayerLeave
  (params (ButtonID :type Integer))
  ;[1 1 1] 弹框确认是否离开场景
  (Utilities|FlowControl|Sequence
    (:then_0
      (switch int ButtonID
        (:Default
          (Utilities|FlowControl|Delay 3.0)
          (Utilities|FlowControl|DoOnce false :!label _label ; enters at Reset
            (:Completed
              (bind _popselect (CallFunction|ShowPopSelectWindow "是否撤退?" (Utilities|Map|MakeMap "是" true "否" true)))
              (EventDispatchers|BindEventtoSelectButton _popselect (delegate Custom|CE_SelectWhenPlayerLeave)))))
        (:0
          (Utilities|FlowControl|Sequence
            (:then_0
              ;[1 1 1] PlayerLeave
              (Default|EventPlayerLeaveGuildPoint (Variables|Default|GetGameModeWM))
              (CallFunction|ShowGameInfo (Utilities|Text|ToText(String) (Utilities|String|JoinStringArray (Utilities|Array|MakeArray "离开" "Guild" (Utilities|String|ToString(Integer) (Variables|Default|GetGuildID))) " "))))
            (:then_1
              (goto _label Reset))))))))

(event EventBeginPlay
  (bind _asbp_game_mode_world_map (Utilities|Casting|CastToBP_GameMode_WorldMap (Game|GetGameMode)))
  (Variables|Default|SetGameModeWM _asbp_game_mode_world_map)
  (|CallParentFunction))

(event Collision|EventActorBeginOverlap
  (params (OtherActor :type Actor%20Object%20Reference)))

(event EventCEPlayerEnter
  (Default|EventPlayerEnterGuildPoint (Variables|Default|GetGameModeWM) self))

(event EventCEPlayerLeave
  (Default|CEPlayerExitGuildPoint (Variables|Default|GetGameModeWM) self))

(event EventTick
  (params (DeltaSeconds :type Float%20%28single-precision%29)))

(fn ConstructionScript
  (bind _billboard (Variables|Default|GetBillboard))
  (|CallParentFunction)
  (if (<= (Variables|Default|GetGuildID) 21)
    (Variables|/Script/Engine.BillboardComponent|SetSprite _billboard "/Game/MyGame/UI/Icon/Icon_Build_0.Icon_Build_0")
    (else
      (Variables|/Script/Engine.BillboardComponent|SetSprite _billboard "/Game/MyGame/UI/Icon/Icon_Build_1.Icon_Build_1")))
  (bind _outactors (Actor|GetAllActorswithTag (Utilities|String|StringToName (Utilities|String|JoinStringArray (Utilities|Array|MakeArray "Guild" (Utilities|String|ToString(Integer) (Variables|Default|GetGuildID))) "_"))))
  (bind _output_get (Variables|Default|SetMovePointArray _outactors))
  (Development|PrintString (Utilities|String|ToString(Integer) (Utilities|Array|Length _output_get))))

(fn BuildGuildShpere
  (params (LinearColor :type Linear%20Color%20Structure%20%28by%20ref%29) (ScaleValue :type Float%20%28single-precision%29))
  (bind _returnvalue (Transformation|GetActorLocation))
  (bind _sphere_0 (Variables|Default|GetSphere_0))
  (bind (_x _y) (Math|Vector|BreakVector _returnvalue))
  (Rendering|Material|SetMaterial _sphere_0 0 "/Game/MyGame/GameMode/Material/M_GuildSphere_Base_Inst.M_GuildSphere_Base_Inst")
  (Rendering|Material|SetVectorParameterValueonMaterials _sphere_0 "MainColor" (Math|Conversions|ToVector(LinearColor) LinearColor))
  (Transformation|SetRelativeScale3D _sphere_0 (Math|Vector|MakeVector ScaleValue ScaleValue ScaleValue))
  (bind (_outhit _returnvalue_2) (Collision|LineTraceForObjects _returnvalue (Math|Vector|MakeVector _x (+ _y 0.05) -3e+04) (Utilities|Array|MakeArray "ObjectTypeQuery1") false (Utilities|Array|MakeArray 0) "None"))
  (if _returnvalue_2
    (Transformation|SetActorLocation (.Location (Collision|BreakHitResult _outhit)) false false)
    (else
      (Development|PrintString "Hello"))))

(fn IsPlayerinThisGuild?
  (params (InActor :type Actor%20Object%20Reference))
  (bind _asbp_game_mode_world_map (Utilities|Casting|CastToBP_GameMode_WorldMap (Game|GetGameMode))
    (:then
      _)
    (:CastFailed
      _))
  (return (and (== InActor (Game|Player|GetPlayerPawn 0)) (== (Variables|/Game/MyGame/GameMode/Buleprint/BP_GameMode_WorldMap.BP_GameMode_WorldMap_C|GetCurrGuildPoint _asbp_game_mode_world_map) self))))

(fn AddCharacterinThisGuild
  (params (GuildID :type Integer) (Native :type Boolean) (Mission :type Boolean) (IsTeam :type Boolean) (InEntrance :type Boolean))
  (bind _loc_characterbasearray (LocalVariables|GetLoc_CharacterBaseArray))
  (Utilities|FlowControl|Sequence
    (:then_0
      (LocalVariables|SetLoc_CharacterGuildID GuildID))
    (:then_1
      (for (_array_element _array_index) (.CharacterDataArray (Utilities|Struct|BreakS_GuildData (Utilities|Array|Get(acopy) (Variables|/Game/MyGame/GameMode/Buleprint/BP_SaveGame.BP_SaveGame_C|GetGuildDataArray (CallFunction|GetMySaveGame)) (LocalVariables|GetLoc_CharacterGuildID))))
        (if (CallFunction|IsCharacterCanAdd _array_element Mission Native)
          (bind _returnvalue (AI|SpawnAIFromClass "/Game/MyGame/GameMode/Character/JYH_BP_Character_AI.JYH_BP_Character_AI_C" 0 "0, 0, 0" "0, 0, 0" true))
          (bind _asjyh_bp_character_ai (Utilities|Casting|CastToJYH_BP_Character_AI _returnvalue))
          (Utilities|Struct|SetmembersinS_CharacterData (Utilities|Array|Get(acopy) (.CharacterDataArray (Utilities|Struct|BreakS_GuildData (Utilities|Array|Get(acopy) (Variables|/Game/MyGame/GameMode/Buleprint/BP_SaveGame.BP_SaveGame_C|GetGuildDataArray (CallFunction|GetMySaveGame)) (LocalVariables|GetLoc_CharacterGuildID)))) _array_index) _asjyh_bp_character_ai)
          (Utilities|Array|Add (Variables|/Script/Engine.Actor|GetTags _asjyh_bp_character_ai) (Utilities|String|StringToName (Utilities|String|ToString(Integer) (LocalVariables|GetLoc_CharacterGuildID))))
          (Default|SetCharacterAIConfig _asjyh_bp_character_ai self (LocalVariables|GetLoc_CharacterGuildID) _array_index)
          (Transformation|SetActorTransform _asjyh_bp_character_ai (Math|Transform|MakeTransform (+ (Math|Vector|SelectVector (CallFunction|FindEntranceLocation) (CallFunction|SelectNewCharacterLocation _array_index) InEntrance) "0, 0,300.000000")))
          (Utilities|Array|Add (LocalVariables|GetLoc_CharacterBaseArray) _asjyh_bp_character_ai)
          (bind _asbp_game_mode_world_map (Utilities|Casting|CastToBP_GameMode_WorldMap (Game|GetGameMode)))
          (Default|EventCharacterEnter _asbp_game_mode_world_map _asjyh_bp_character_ai)))
      (if IsTeam
        (for _array_element_2 _loc_characterbasearray
          (Variables|/Game/MyGame/GameMode/Character/JYH_BP_Character_Base.JYH_BP_Character_Base_C|SetTeam _array_element_2 _loc_characterbasearray))))))

(fn FindEntranceLocation
  (bind _entrancearray (Variables|Default|GetEntranceArray))
  (bind _output (Utilities|Array|Get(acopy) _entrancearray))
  (if (> (Utilities|Array|Length _entrancearray) 0)
    (if (Utilities|IsValid _output)
      (return (.RandomLocation (AI|Navigation|GetRandomReachablePointinRadius (Transformation|GetActorLocation _output) 3e+02 0 0)))
      (else
        _)))
  (return (.RandomLocation (AI|Navigation|GetRandomReachablePointinRadius (Transformation|GetActorLocation) (Variables|Default|GetRadius) 0 0))))

(fn IsCharacterCanAdd
  (params (S_CharacterData :type S%20Character%20Data%20Structure%20%28by%20ref%29) (Mission :type Boolean) (Native :type Boolean))
  (bind (_surname _name _camp _moral _exp _constitution _strength _dexterous _intelligence _currhealth _occid _ismission_ _itemmap _equipmap _gestmap _skillmap _isplayer _character) (Utilities|Struct|BreakS_CharacterData S_CharacterData))
  (return (Math|Boolean|ANDBoolean (or (and Native (not _ismission_)) (and Mission _ismission_)) (> _currhealth 0.0) (not _isplayer) (== _character 0))))

(fn SelectNewCharacterLocation
  (params (ChildID :type Integer))
  (bind _returnvalue (Transformation|GetActorLocation))
  (bind _aifixedpointarrayarray (Variables|Default|GetAIFixedPointArrayArray))
  (bind _movepointarray (Variables|Default|GetMovePointArray))
  (bind _returnvalue_2 (Utilities|Array|LastIndex _movepointarray))
  (bind _output (Utilities|Array|Get(acopy) _aifixedpointarrayarray ChildID))
  (bind _actorarray (Utilities|Struct|BreakS_ActorArray _output))
  (bind _returnvalue_3 (Math|Random|RandomIntegerinRange 0 _returnvalue_2))
  (bind _output_2 (Utilities|Array|Get(acopy) _movepointarray _returnvalue_3))
  (if (Utilities|Array|IsValidIndex _aifixedpointarrayarray ChildID)
    (if (> (Utilities|Array|Length _actorarray) 0)
      (return (.RandomLocation (AI|Navigation|GetRandomReachablePointinRadius (Transformation|GetActorLocation (Utilities|Array|Get(acopy) _actorarray (Math|Random|RandomIntegerinRange 0 (Utilities|Array|LastIndex _actorarray)))) 1e+02 0 0)))
      (else
        _)))
  (if (> (Utilities|Array|Length _movepointarray) 0)
    (Utilities|IsValid _output_2
      (:Is%20Valid
        (return (.RandomLocation (AI|Navigation|GetRandomReachablePointinRadius (Transformation|GetActorLocation _output_2) 6e+02 0 0))))
      (:Is%20Not%20Valid
        _)))
  (bind (_outhit _returnvalue_4) (Collision|LineTraceByChannel _returnvalue (+ _returnvalue "0, 0,-1000.000000") "TraceTypeQuery1" false (Utilities|Array|MakeArray) "None" true "(R=1.000000,G=0.000000,B=0.000000,A=1.000000)" "(R=0.000000,G=1.000000,B=0.000000,A=1.000000)" 5e+02))
  (return (Math|Vector|SelectVector (.RandomLocation (AI|Navigation|GetRandomReachablePointinRadius (.Location (Collision|BreakHitResult _outhit)) 2e+02 0 0)) _returnvalue _returnvalue_4)))